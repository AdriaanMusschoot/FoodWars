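; BP_Table is a table that holds one carried item dropped onto it.
; On BeginPlay it hands its Top mesh to BPCInteractible and binds HandleObject to that component's drop-off event.
; When empty, HandleObject accepts only actors with a BPC_PickUpComponent, moves them to the table location plus AnchorPoint, and stores them as Content.
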(event Custom|HandleObject
  (params (HeldObject :type Actor%20Object%20Reference))
  (Utilities|IsValid (Variables|Default|GetContent)
    (:Is%20Not%20Valid
      (Utilities|IsValid (Actor|GetComponentbyClass HeldObject "/Game/Ingredients/BPC_PickUpComponent.BPC_PickUpComponent_C")
        (:Is%20Valid
          (Transformation|SetActorLocation HeldObject (+ (Variables|Default|GetAnchorPoint) (Transformation|GetActorLocation)) false false)
          (Variables|Default|SetContent HeldObject))))))

(event EventBeginPlay
  (Variables|/Game/Furnace/BPC_Interactible.BPC_Interactible_C|SetMeshToSet (Variables|Default|GetBPC_Interactible) (Variables|Default|GetTop))
  (EventDispatchers|BindEventtoDropOffItem (Variables|Default|GetBPC_Interactible) (delegate Custom|HandleObject)))

(fn ConstructionScript)