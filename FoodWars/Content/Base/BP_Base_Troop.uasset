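; Base character for two-team troops that head for the opposing tagged tower and fight enemy troops along the way.
; PlayerIndex selects the tower and team tag, while sight-collider overlaps track enemies and set MoveTarget to the nearer of closest enemy or tower.
; Tick deals timed Health hits to the closest enemy in range, or to the tower when none exists.
; A timer-reset BodyColor change provides a temporary tint.
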(event OnComponentBeginOverlap(SightRangeCollider)
  (params (OverlappedComponent :type Primitive%20Component%20Object%20Reference) (OtherActor :type Actor%20Object%20Reference) (OtherComp :type Primitive%20Component%20Object%20Reference) (OtherBodyIndex :type Integer) (bFromSweep :type Boolean) (SweepResult :type Hit%20Result%20Structure%20%28by%20ref%29))
  (bind _enemiesinsight (Variables|Default|GetEnemiesInSight))
  (bind _asbp_base_troop (Utilities|Casting|CastToBP_Base_Troop OtherActor))
  (bind _areindifferentteams (CallFunction|CheckTags _asbp_base_troop))
  (if _areindifferentteams
    (Utilities|Array|Add _enemiesinsight _asbp_base_troop)
    (CallFunction|GetClosestEnemy _enemiesinsight)
    (CallFunction|CheckUpdateTarget)
    ;[1 0.9131 0.4233] debuging
    (for _array_element _enemiesinsight
      (Development|PrintString (Utilities|GetDisplayName _array_element) true true "(R=1.000000,G=0.607181,B=0.000000,A=1.000000)"))))

(event OnComponentEndOverlap(SightRangeCollider)
  (params (OverlappedComponent :type Primitive%20Component%20Object%20Reference) (OtherActor :type Actor%20Object%20Reference) (OtherComp :type Primitive%20Component%20Object%20Reference) (OtherBodyIndex :type Integer))
  (bind _enemiesinsight (Variables|Default|GetEnemiesInSight))
  (bind _asbp_base_troop (Utilities|Casting|CastToBP_Base_Troop OtherActor))
  (bind _areindifferentteams (CallFunction|CheckTags _asbp_base_troop))
  (if _areindifferentteams
    (Utilities|Array|RemoveItem _enemiesinsight _asbp_base_troop)
    (CallFunction|GetClosestEnemy _enemiesinsight)
    (CallFunction|CheckUpdateTarget)
    ;[1 0.9131 0.4233] debuging
    (if (> (Utilities|Array|Length _enemiesinsight) 0)
      (for _array_element _enemiesinsight
        (Development|PrintString (Utilities|GetDisplayName _array_element) true true "(R=1.000000,G=0.607181,B=0.000000,A=1.000000)"))
      (else
        (Development|PrintString "No enemies in sight" true true "(R=1.000000,G=0.000000,B=0.072013,A=1.000000)")))))

(event EventBeginPlay
  (bind _returnvalue (Rendering|Material|CreateDynamicMaterialInstance (Actor|GetComponentbyClass "/Script/Engine.StaticMeshComponent") 0 0 "None" :!class /Script/Engine.PrimitiveComponent))
  (bind _returnvalue_2 (Rendering|Material|GetVectorParameterValue _returnvalue "BodyColor" :!class /Script/Engine.MaterialInstanceDynamic))
  (Variables|ColorChange|SetOriginalColor _returnvalue_2)
  (Variables|Default|SetMoveToStopRange (- (Variables|Attack|GetAttackRange) 25.0))
  (Variables|Attack|SetAttackTimer (Variables|Attack|GetAttackSpeed))
  (Variables|/Script/Engine.CharacterMovementComponent|SetMaxWalkSpeed (Variables|Character|GetCharacterMovement) (Variables|Default|GetSpeed))
  (if (== (Variables|Default|GetPlayerIndex) 0)
    (bind _outactors (Actor|GetAllActorswithTag "Tower2"))
    (bind _output_get (Variables|Default|SetMoveTarget (Utilities|Array|Get(acopy) _outactors)))
    (Variables|Default|SetTargetTower _output_get)
    (Variables|Default|SetBehavior "NewEnumerator0")
    (else
      (bind _outactors_2 (Actor|GetAllActorswithTag "Tower1"))
      (bind _output_get_2 (Variables|Default|SetMoveTarget (Utilities|Array|Get(acopy) _outactors_2)))
      (Variables|Default|SetTargetTower _output_get_2)
      (Variables|Default|SetBehavior "NewEnumerator0"))))

(event Collision|EventActorBeginOverlap
  (params (OtherActor :type Actor%20Object%20Reference)))

(event EventTick
  (params (DeltaSeconds :type Float%20%28single-precision%29))
  (bind _targettower (Variables|Default|GetTargetTower))
  (bind _attackrange (Variables|Attack|GetAttackRange))
  (bind _targettower_2 (Variables|Default|GetTargetTower))
  (bind _attackrange_2 (Variables|Attack|GetAttackRange))
  (bind _returnvalue (Actor|GetComponentbyClass _targettower "/Game/Troops/Health.Health_C"))
  (Utilities|IsValid (Variables|ClosestEnemy|GetClosets%20Enemy)
    (:Is%20Valid
      (if (<= (Class|KismetMathLibrary|VectorDistanceSquared (Transformation|GetActorLocation (Variables|ClosestEnemy|GetClosets%20Enemy)) (Transformation|GetActorLocation self)) (* _attackrange_2 _attackrange_2))
        (bind _output_get (Variables|Attack|SetAttackTimer (- (Variables|Attack|GetAttackTimer) DeltaSeconds)))
        (if (<= _output_get 0.0)
          (Variables|Attack|SetAttackTimer (Variables|Attack|GetAttackSpeed))
          (Default|Hit (Variables|BP_Base_Troop_C|GetHealth (Variables|ClosestEnemy|GetClosets%20Enemy)) (Variables|Attack|GetDamage) self))))
    (:Is%20Not%20Valid
      (Utilities|IsValid _targettower_2
        (:Is%20Valid
          (if (<= (Class|KismetMathLibrary|VectorDistanceSquared (Transformation|GetActorLocation _targettower_2) (Transformation|GetActorLocation self)) (* _attackrange _attackrange))
            (bind _output_get_2 (Variables|Attack|SetAttackTimer (- (Variables|Attack|GetAttackTimer) DeltaSeconds)))
            (if (<= _output_get_2 0.0)
              (Variables|Attack|SetAttackTimer (Variables|Attack|GetAttackSpeed))
              (Utilities|IsValid _returnvalue
                (:Is%20Valid
                  (Default|Hit _returnvalue (Variables|Attack|GetDamage) self))))))))))

(fn ConstructionScript)

(fn SetPlayerIdex
  (params (Index :type Integer))
  (bind _output_get (Variables|Default|SetPlayerIndex Index))
  (if (== _output_get 0)
    (bind _outactors (Actor|GetAllActorswithTag "Tower2"))
    (bind _output_get_2 (Variables|Default|SetMoveTarget (Utilities|Array|Get(acopy) _outactors)))
    (Variables|Default|SetTargetTower _output_get_2)
    (Variables|Default|SetBehavior "NewEnumerator0")
    (Variables|Default|SetTags self (Utilities|Array|MakeArray "Team1"))
    (else
      (bind _outactors_2 (Actor|GetAllActorswithTag "Tower1"))
      (bind _output_get_3 (Variables|Default|SetMoveTarget (Utilities|Array|Get(acopy) _outactors_2)))
      (Variables|Default|SetTargetTower _output_get_3)
      (Variables|Default|SetBehavior "NewEnumerator0")
      (Variables|Default|SetTags self (Utilities|Array|MakeArray "Team2")))))

(fn GetClosestEnemy
  (params (EnemyArray :type Array%20of%20BP%20Base%20Troop%20Object%20References))
  (for _array_element EnemyArray
    (if (not (Variables|BP_Base_Troop_C|GetIsMarkedForDestroy _array_element))
      (if (< (Class|KismetMathLibrary|VectorDistanceSquared (Transformation|GetActorLocation _array_element) (Transformation|GetActorLocation self)) (Variables|ClosestEnemy|GetClosestDistance))
        (Variables|ClosestEnemy|SetClosestDistance (Class|KismetMathLibrary|VectorDistanceSquared (Transformation|GetActorLocation _array_element) (Transformation|GetActorLocation self)))
        (Variables|ClosestEnemy|SetClosets%20Enemy _array_element))))
  (return (Variables|ClosestEnemy|GetClosets%20Enemy)))

(fn CheckTags
  (params (NewParam :type BP%20Base%20Troop%20Object%20Reference))
  (bind _tags (Variables|Default|GetTags))
  (bind _tags_2 (Variables|/Script/Engine.Actor|GetTags NewParam))
  (bind _tags_3 (Variables|Default|GetTags))
  (bind _tags_4 (Variables|/Script/Engine.Actor|GetTags NewParam))
  (bind _returnvalue (Utilities|Array|ContainsItem _tags "Team2"))
  (bind _returnvalue_2 (Utilities|Array|ContainsItem _tags_2 "Team1"))
  (bind _returnvalue_3 (Utilities|Array|ContainsItem _tags_3 "Team1"))
  (bind _returnvalue_4 (Utilities|Array|ContainsItem _tags_4 "Team2"))
  (bind _returnvalue_5 (and _returnvalue _returnvalue_2))
  (bind _returnvalue_6 (and _returnvalue_3 _returnvalue_4))
  (bind _returnvalue_7 (or _returnvalue_6 _returnvalue_5))
  (if _returnvalue_7
    (return _returnvalue_7)))

(fn CheckUpdateTarget
  (bind _closets_enemy (Variables|ClosestEnemy|GetClosets%20Enemy))
  (Utilities|IsValid (Variables|ClosestEnemy|GetClosets%20Enemy)
    (:Is%20Valid
      (if (not (Variables|BP_Base_Troop_C|GetIsMarkedForDestroy _closets_enemy))
        (if (< (Class|KismetMathLibrary|VectorDistanceSquared (Transformation|GetActorLocation _closets_enemy) (Transformation|GetActorLocation self)) (Class|KismetMathLibrary|VectorDistanceSquared (Transformation|GetActorLocation (Variables|Default|GetTargetTower)) (Transformation|GetActorLocation self)))
          (Variables|Default|SetMoveTarget (Variables|ClosestEnemy|GetClosets%20Enemy))
          (else
            (Variables|Default|SetMoveTarget (Variables|Default|GetTargetTower))))
        (else
          (Variables|Default|SetMoveTarget (Variables|Default|GetTargetTower)))))
    (:Is%20Not%20Valid
      (Variables|Default|SetMoveTarget (Variables|Default|GetTargetTower)))))

(fn ChangeMeshColor
  (params (NewColor :type Linear%20Color%20Structure))
  (for _array_element (Actor|GetComponentsByClass "/Script/Engine.StaticMeshComponent")
    (Rendering|Material|SetVectorParameterValueonMaterials _array_element "BodyColor" (Math|Conversions|ToVector(LinearColor) NewColor))
    (Utilities|Time|SetTimerbyFunctionName 0 "ResetMeshColor" (Variables|ColorChange|GetColorChangeTime))))

(fn ResetMeshColor
  (for _array_element (Actor|GetComponentsByClass "/Script/Engine.StaticMeshComponent")
    (Rendering|Material|SetVectorParameterValueonMaterials _array_element "BodyColor" (Math|Conversions|ToVector(LinearColor) (Variables|ColorChange|GetOriginalColor)))))