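; Player cook character that moves, picks up and drops items, feeds ingredients to furnaces and throws dishes.
; An overlap collider tracks nearby pickups and furnaces, marking the closest furnace interactible.
; Interacting drops the held item, or collects the closest furnace's dish, falling back to the nearest pickup.
; While aiming, movement input is nearly zeroed to set the throw direction, which Tick passes to the held item's throw component.
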(event OnComponentBeginOverlap(PickUpCollider)
  (params (OverlappedComponent :type Primitive%20Component%20Object%20Reference) (OtherActor :type Actor%20Object%20Reference) (OtherComp :type Primitive%20Component%20Object%20Reference) (OtherBodyIndex :type Integer) (bFromSweep :type Boolean) (SweepResult :type Hit%20Result%20Structure%20%28by%20ref%29))
  (Utilities|IsValid (Actor|GetComponentbyClass OtherActor "/Game/Ingredients/BPC_PickUpComponent.BPC_PickUpComponent_C")
    (:Is%20Valid
      (Utilities|Array|Add (Variables|Default|GetPickUpableInRange) OtherActor))
    (:Is%20Not%20Valid
      (bind _asbp_furnace (Utilities|Casting|CastToBP_Furnace OtherActor))
      (Utilities|IsValid (Variables|Default|GetClosestFurnace)
        (:Is%20Valid
          (Default|Interactible (Variables|Default|GetClosestFurnace) false))
        (:Is%20Not%20Valid
          _))
      (Utilities|Array|Add (Variables|Default|GetFurnacesInRange) _asbp_furnace)
      (bind _closestactor (CallFunction|GetClosestObject (Variables|Default|GetFurnacesInRange)))
      (bind _asbp_furnace_2 (Utilities|Casting|CastToBP_Furnace _closestactor)
        (:then
          _)
        (:CastFailed
          _))
      (bind _output_get (Variables|Default|SetClosestFurnace _asbp_furnace_2))
      (Default|Interactible _output_get true))))

(event OnComponentEndOverlap(PickUpCollider)
  (params (OverlappedComponent :type Primitive%20Component%20Object%20Reference) (OtherActor :type Actor%20Object%20Reference) (OtherComp :type Primitive%20Component%20Object%20Reference) (OtherBodyIndex :type Integer))
  (Utilities|IsValid (Actor|GetComponentbyClass OtherActor "/Game/Ingredients/BPC_PickUpComponent.BPC_PickUpComponent_C")
    (:Is%20Valid
      (Utilities|Array|RemoveItem (Variables|Default|GetPickUpableInRange) OtherActor))
    (:Is%20Not%20Valid
      (bind _asbp_furnace (Utilities|Casting|CastToBP_Furnace OtherActor))
      (Default|Interactible _asbp_furnace false)
      (Utilities|Array|RemoveItem (Variables|Default|GetFurnacesInRange) _asbp_furnace)
      (bind _closestactor (CallFunction|GetClosestObject (Variables|Default|GetFurnacesInRange)))
      (bind _asbp_furnace_2 (Utilities|Casting|CastToBP_Furnace _closestactor)
        (:then
          (bind _output_get (Variables|Default|SetClosestFurnace _asbp_furnace_2))
          (Default|Interactible _output_get true))
        (:CastFailed
          (Variables|Default|SetClosestFurnace 0))))))

(event Custom|Move
  (params (Axis%20Value :type Vector%202D%20Structure))
  (bind _result (Math|Float|NegateFloat (.x Axis%20Value))
    (:%20%20
      (if (Variables|Default|GetIsAiming)
        (Pawn|Input|AddMovementInput (Math|Vector|MakeVector _result (.y Axis%20Value) 0.0) 1e-05 false)
        (Variables|Default|SetCachedThrowDirection (Math|Vector|MakeVector _result (.y Axis%20Value) 0.0))
        (else
          (Pawn|Input|AddMovementInput (Math|Vector|MakeVector _result (.y Axis%20Value) 0.0) 1.0 false))))))

(event Custom|StartAiming
  (bind _pickupinpossession (Variables|Default|GetPickUpInPossession))
  (Utilities|IsValid _pickupinpossession
    (:Is%20Valid
      (Utilities|IsValid (Actor|GetComponentbyClass _pickupinpossession "/Game/Dish/BPC_ThrowComponent.BPC_ThrowComponent_C")
        (:Is%20Valid
          (Variables|Default|SetIsAiming true))))))

(event Custom|StartThrow
  (bind _pickupinpossession (Variables|Default|GetPickUpInPossession))
  (Utilities|IsValid _pickupinpossession
    (:Is%20Valid
      (Utilities|IsValid (Actor|GetComponentbyClass _pickupinpossession "/Game/Dish/BPC_ThrowComponent.BPC_ThrowComponent_C")
        (:Is%20Valid
          (Variables|Default|SetIsAiming false)
          (CallFunction|ThrowDish self))))))

(event EventBeginPlay)

(event Collision|EventActorBeginOverlap
  (params (OtherActor :type Actor%20Object%20Reference)))

(event EventTick
  (params (DeltaSeconds :type Float%20%28single-precision%29))
  (bind _pickupinpossession (Variables|Default|GetPickUpInPossession))
  (bind _returnvalue (Actor|GetComponentbyClass _pickupinpossession "/Game/Dish/BPC_ThrowComponent.BPC_ThrowComponent_C"))
  (if (Variables|Default|GetIsAiming)
    (Utilities|IsValid _pickupinpossession
      (:Is%20Valid
        (Utilities|IsValid _returnvalue
          (:Is%20Valid
            (Default|AimThrow _returnvalue (Variables|Default|GetCachedThrowDirection) self)))))))

(fn ConstructionScript)

(fn LookforPickUp
  (Utilities|IsValid (Variables|Default|GetClosestFurnace)
    (:Is%20Valid
      (bind _dish (Default|CollectDish (Variables|Default|GetClosestFurnace)))
      (Utilities|IsValid _dish
        (:Is%20Valid
          (Default|GrabItem (Actor|GetComponentbyClass _dish "/Game/Ingredients/BPC_PickUpComponent.BPC_PickUpComponent_C"))
          (CallFunction|AttachActorPoint self _dish))
        (:Is%20Not%20Valid
          (bind _closestactor (CallFunction|GetClosestObject (Variables|Default|GetPickUpableInRange) :!label _label))
          (Utilities|IsValid _closestactor
            (:Is%20Valid
              (Utilities|IsValid (Actor|GetComponentbyClass _closestactor "/Game/Ingredients/BPC_PickUpComponent.BPC_PickUpComponent_C")
                (:Is%20Valid
                  (Default|GrabItem (Actor|GetComponentbyClass _closestactor "/Game/Ingredients/BPC_PickUpComponent.BPC_PickUpComponent_C")))
                (:Is%20Not%20Valid
                  _))
              (CallFunction|AttachActorPoint self _closestactor))))))
    (:Is%20Not%20Valid
      (goto _label))))

(fn DropIngredient
  (Transformation|DetachFromActor (Variables|Default|GetPickUpInPossession) "KeepWorld" "KeepRelative" "KeepRelative")
  (Default|DropItem (Actor|GetComponentbyClass (Variables|Default|GetPickUpInPossession) "/Game/Ingredients/BPC_PickUpComponent.BPC_PickUpComponent_C"))
  (Utilities|IsValid (Variables|Default|GetClosestFurnace)
    (:Is%20Valid
      (bind _asbp_ingredient (Utilities|Casting|CastToBP_Ingredient (Variables|Default|GetPickUpInPossession))
        (:then
          (Default|HandleIngredient (Variables|Default|GetClosestFurnace) _asbp_ingredient))
        (:CastFailed
          _)))
    (:Is%20Not%20Valid
      _))
  (Variables|Default|SetPickUpInPossession 0))

(fn TriggerInteract
  (Utilities|IsValid (Variables|Default|GetPickUpInPossession)
    (:Is%20Valid
      (CallFunction|DropIngredient))
    (:Is%20Not%20Valid
      (CallFunction|LookforPickUp))))

(fn GetClosestObject
  (params (ObjectsInRange :type Array%20of%20Actor%20Object%20References))
  (for _array_element ObjectsInRange
    (if (< (Math|Vector|Distance(Vector) (Transformation|GetActorLocation _array_element) (Transformation|GetActorLocation self)) (LocalVariables|GetMinimalDistance))
      (LocalVariables|SetMinimalDistance (Math|Vector|Distance(Vector) (Transformation|GetActorLocation _array_element) (Transformation|GetActorLocation self)))
      (LocalVariables|SetTempClosestActor _array_element)))
  (return (LocalVariables|GetTempClosestActor)))

(fn AttachActorPoint
  (params (Actor :type Actor%20Object%20Reference))
  (Transformation|SetActorLocation Actor (Variables|Default|GetPickUpAnchorPoint) false false)
  (bind _returnvalue (Transformation|AttachActorToActor Actor self "None" "KeepRelative" "KeepRelative" "KeepRelative" true))
  (if _returnvalue
    (Variables|Default|SetPickUpInPossession Actor)))

(fn ThrowDish
  (Utilities|IsValid (Actor|GetComponentbyClass (Variables|Default|GetPickUpInPossession) "/Game/Ingredients/BPC_PickUpComponent.BPC_PickUpComponent_C")
    (:Is%20Valid
      (Transformation|DetachFromActor (Variables|Default|GetPickUpInPossession) "KeepWorld" "KeepRelative" "KeepRelative")
      (Default|DropItem (Actor|GetComponentbyClass (Variables|Default|GetPickUpInPossession) "/Game/Ingredients/BPC_PickUpComponent.BPC_PickUpComponent_C"))
      (Default|InitiateThrow (Actor|GetComponentbyClass (Variables|Default|GetPickUpInPossession) "/Game/Dish/BPC_ThrowComponent.BPC_ThrowComponent_C") self)
      (Variables|Default|SetPickUpInPossession 0))))