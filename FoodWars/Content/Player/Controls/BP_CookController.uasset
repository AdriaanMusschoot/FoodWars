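; BP_CookController is a player controller that routes Enhanced Input to the controlled cook character.
; On BeginPlay it adds the IMC_Cook mapping context, then casts the controlled pawn to BP_Cook and stores it as PlayerReference.
; The move and interact input actions are forwarded to that reference's Move and TriggerInteract functions, guarded by validity checks.
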(event Input|EnhancedActionEvents|EnhancedInputActionIA_CMove
  (params (ActionValue :type Vector%202D%20Structure) (ElapsedSeconds :type Float%20%28double-precision%29) (TriggeredSeconds :type Float%20%28double-precision%29) (InputAction :type Input%20Action%20Object%20Reference :default "/Game/Player/Controls/IA_CMove.IA_CMove"))
  (bind _playerreference (Variables|Default|GetPlayerReference))
  (Utilities|IsValid _playerreference
    (:Is%20Valid
      (Default|Move _playerreference ActionValue))))

(event Input|EnhancedActionEvents|EnhancedInputActionIA_Interact
  (params (ActionValue :type Boolean) (ElapsedSeconds :type Float%20%28double-precision%29) (TriggeredSeconds :type Float%20%28double-precision%29) (InputAction :type Input%20Action%20Object%20Reference :default "/Game/Player/Controls/IA_Interact.IA_Interact"))
  (bind _playerreference (Variables|Default|GetPlayerReference))
  (Utilities|IsValid _playerreference
    (:Is%20Valid
      (Default|TriggerInteract _playerreference))))

(event EventBeginPlay
  (bind _returnvalue (PlayerController|LocalPlayerSubsystems|GetEnhancedInputLocalPlayerSubsystem))
  (Utilities|IsValid _returnvalue
    (:Is%20Valid
      (Input|AddMappingContext _returnvalue "/Game/Player/Controls/IMC_Cook.IMC_Cook" 0 "(bIgnoreAllPressedKeysUntilRelease=True,bForceImmediately=False,bNotifyUserSettings=False)")
      (bind _asbp_cook (Utilities|Casting|CastToBP_Cook (Pawn|GetControlledPawn)))
      (Variables|Default|SetPlayerReference _asbp_cook))))

(event EventTick
  (params (DeltaSeconds :type Float%20%28single-precision%29)))

(fn ConstructionScript)