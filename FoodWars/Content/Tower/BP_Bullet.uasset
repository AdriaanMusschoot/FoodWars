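; BP_Bullet is a tower-defense homing projectile that chases its assigned Target and damages enemy troops.
; Each tick it moves with sweep toward the target's location at BulletSpeed, destroying itself if the target becomes invalid.
; A sphere overlap with the capsule of a BP_Base_Troop on another team calls Hit on its Health component with Damage, prints debug text, and destroys the bullet.
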(event OnComponentBeginOverlap(Sphere)
  (params (OverlappedComponent :type Primitive%20Component%20Object%20Reference) (OtherActor :type Actor%20Object%20Reference) (OtherComp :type Primitive%20Component%20Object%20Reference) (OtherBodyIndex :type Integer) (bFromSweep :type Boolean) (SweepResult :type Hit%20Result%20Structure%20%28by%20ref%29))
  (bind _asbp_base_troop (Utilities|Casting|CastToBP_Base_Troop OtherActor))
  (Utilities|Casting|CastToCapsuleComponent OtherComp)
  (if (!= (Variables|/Game/Base/BP_Base_Troop.BP_Base_Troop_C|GetPlayerIndex _asbp_base_troop) (Variables|Default|GetTeamId))
    (Utilities|IsValid (Actor|GetComponentbyClass _asbp_base_troop "/Game/Troops/Health.Health_C")
      (:Is%20Valid
        (Default|Hit (Actor|GetComponentbyClass _asbp_base_troop "/Game/Troops/Health.Health_C") (Variables|Default|GetDamage))
        (Development|PrintText "Hello IM DYING HELP (bullet)")
        (Actor|DestroyActor)))))

(event EventBeginPlay)

(event Collision|EventActorBeginOverlap
  (params (OtherActor :type Actor%20Object%20Reference)))

(event EventTick
  (params (DeltaSeconds :type Float%20%28single-precision%29))
  (bind _target (Variables|Default|GetTarget))
  (Utilities|IsValid _target
    (:Is%20Valid
      (Transformation|AddActorWorldOffset (* (Math|Vector|Normalize (- (Transformation|GetActorLocation _target) (Transformation|GetActorLocation self))) (Variables|Default|GetBulletSpeed) (Utilities|Time|GetWorldDeltaSeconds)) true))
    (:Is%20Not%20Valid
      (Actor|DestroyActor))))

(fn ConstructionScript)