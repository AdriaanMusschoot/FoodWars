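; Ingredient delivery actor that spawns a row of ingredient boxes in the level.
; On BeginPlay, it spawns one box per class in ClassesToSpawn, stepping by an offset from a spawn point, and stores each in IngredientBoxes.
; A Sequencer event can trigger the same spawn again, adding more boxes without clearing existing ones.
; Timed refilling of all stored boxes is present but unconnected to Tick, so it never runs.
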(event EventBeginPlay
  (Variables|Default|SetDeliveryTimeLeft (Variables|Default|GetDeliveryTime))
  (CallFunction|SpawnAllBoxes))

(event Collision|EventActorBeginOverlap
  (params (OtherActor :type Actor%20Object%20Reference)))

(event EventTick
  (params (DeltaSeconds :type Float%20%28single-precision%29)))

(event Custom|CallSpawnBoxes
  (CallFunction|SpawnAllBoxes))

(fn ConstructionScript)

(fn SpawnBox
  (params (Location :type Vector) (NewParam :type BP%20Ingredient%20Box%20Class%20Reference))
  (if true
    (bind _returnvalue (Game|SpawnActorfromClass NewParam (Math|Transform|MakeTransform Location) "Undefined" "MultiplyWithRoot" 0 0))
    (Utilities|Array|Add (Variables|Default|GetIngredientBoxes) _returnvalue)
    (else
      (Development|PrintText (Utilities|Text|ToText(String) (Utilities|String|Append "Not enough boxes to spawn!" (Utilities|GetObjectName self)))))))

(fn SpawnAllBoxes
  (for (_array_element _array_index) (Variables|Default|GetClassesToSpawn)
    (CallFunction|SpawnBox (+ (* _array_index (Variables|Default|GetOffset)) (Variables|Default|GetSpawnPoint)) _array_element)))

(fn RefillAllIngredientBoxes
  (for _array_element (Variables|Default|GetIngredientBoxes)
    (Default|RefillIngredients _array_element)))