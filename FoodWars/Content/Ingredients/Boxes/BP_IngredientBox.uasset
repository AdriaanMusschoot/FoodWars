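; BP_IngredientBox is an ingredient container that dispenses a limited stock of ingredient actors and can be refilled.
; BeginPlay fills the stock to its maximum and makes the box the owner of its BPW_ContentAmount widget.
; SpawnIngredient spawns the configured class above the box, applies an upward force, decrements the count and returns the actor, or prints a message when empty.
; RefillIngredients resets the count to the maximum.
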(event EventBeginPlay
  (Variables|Default|SetCurrentIngredientAmount (Variables|Default|GetMaxIngredientAmout))
  (bind _asbpw_content_amount (Utilities|Casting|CastToBPW_ContentAmount (UserInterface|GetUserWidgetObject (Variables|Default|GetWidget))))
  (Variables|/Game/Ingredients/Boxes/BPW_ContentAmount.BPW_ContentAmount_C|SetOwner _asbpw_content_amount self))

(event Collision|EventActorBeginOverlap
  (params (OtherActor :type Actor%20Object%20Reference)))

(event EventTick
  (params (DeltaSeconds :type Float%20%28single-precision%29)))

(fn ConstructionScript)

(fn SpawnIngredient
  (bind _returnvalue (Transformation|GetActorTransform))
  (if (> (Variables|Default|GetCurrentIngredientAmount) 0)
    (bind _returnvalue_2 (Game|SpawnActorfromClass (Variables|Default|GetIngredientClass) (Math|Transform|MakeTransform (+ (.location _returnvalue) "0.000000,0.000000,100.000000") (.rotation _returnvalue) (.scale _returnvalue)) "Undefined" "MultiplyWithRoot" 0 0))
    (Physics|AddForce (Variables|/Game/Ingredients/BP_Ingredient.BP_Ingredient_C|GetMesh _returnvalue_2) "0.000000,0.000000,10.000000" "None" false)
    (bind _result (Math|Integer|DecrementInt (Variables|Default|GetCurrentIngredientAmount))
      (:%20%20
        (Variables|Default|SetCurrentIngredientAmount _result)
        (return _returnvalue_2)))
    (else
      (Development|PrintText (Utilities|Text|ToText(String) (Utilities|String|Append "Not enough ingredients to spawn!" (Utilities|GetObjectName self))))
      (return 0))))

(fn RefillIngredients
  (Variables|Default|SetCurrentIngredientAmount (Variables|Default|GetMaxIngredientAmout)))