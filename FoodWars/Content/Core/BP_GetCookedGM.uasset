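; Game mode for Get Cooked that sets up local multiplayer and the level camera at BeginPlay.
; It loops over the level's PlayerStarts, creating local players with controllers until the player count reaches NrOfPlayers.
; It then points the first player controller's view at the first CameraActor found in the level, if any.
; Tick is disabled, and a debug print of the pawn location is left unconnected.
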(event EventBeginPlay
  (Utilities|FlowControl|Sequence
    (:then_0
      (bind _outactors (Actor|GetAllActorsOfClass "/Script/Engine.PlayerStart"))
      (Utilities|Array|ForEachLoopwithBreak _outactors :!label _label
        (:LoopBody
          (bind _returnvalue (Class|GameModeBase|GetNumPlayers))
          (if (>= _returnvalue (Variables|Default|GetNrOfPlayers))
            (goto _label Break)
            (else
              (bind _returnvalue_2 (Class|GameplayStatics|CreatePlayer -1)))))))
    (:then_1
      (bind _outactors_2 (Actor|GetAllActorsOfClass "/Script/Engine.CameraActor"))
      (if (Utilities|Array|IsNotEmpty _outactors_2)
        (Game|Player|SetViewTargetwithBlend (Game|GetPlayerController 0) (Utilities|Array|Get(acopy) _outactors_2) 0.0 "VTBlend_Linear" 0.0 false)))))

(event EventTick
  (params (DeltaSeconds :type Float%20%28single-precision%29)))

(fn ConstructionScript)