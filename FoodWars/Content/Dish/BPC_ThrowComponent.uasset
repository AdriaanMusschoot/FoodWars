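; BPC_ThrowComponent is an unfinished component for throwing, found among the Dish assets.
; InitiateThrow and AimThrow are stubs that only print a debug string and the aim direction, respectively.
; Disconnected nodes sketch the intended throw: a direction lifted by one minus its length, normalized and scaled by ThrowForce.
; That vector would feed a debug-drawn projectile path prediction and an impulse on a StaticMeshComponent, but neither runs.
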(event EventBeginPlay)

(event EventTick
  (params (DeltaSeconds :type Float%20%28single-precision%29)))

(fn InitiateThrow
  (params (ThrowingPlayer :type BP%20Cook%20Object%20Reference))
  (Development|PrintString "THROWNS;"))

(fn AimThrow
  (params (Direction :type Vector) (ThrowingPlayer :type BP%20Cook%20Object%20Reference))
  (Development|PrintString (Utilities|String|ToString(Vector) Direction)))