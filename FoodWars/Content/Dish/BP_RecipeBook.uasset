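; BP_RecipeBook is a recipe lookup that turns a set of ingredients into a dish.
; GetDish tests recipes through CheckRecipeMatch, which compares CountIngredients tallies for every E_IngredientType, so order is ignored but quantities must match.
; The loop breaks on the first mismatch, so only the first RecipeBook entry is effectively checked.
; A match returns that recipe's ResultingDish, otherwise BP_Dish is returned, with a debug print either way.
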(event EventBeginPlay)

(event Collision|EventActorBeginOverlap
  (params (OtherActor :type Actor%20Object%20Reference)))

(event EventTick
  (params (DeltaSeconds :type Float%20%28single-precision%29)))

(fn ConstructionScript)

(fn GetDish
  (params (Ingredients :type Array%20of%20E_IngredientType%20Enums :default "NewEnumerator0"))
  (bind _array_element (Utilities|Array|ForEachLoopwithBreak (Variables|Default|GetRecipeBook) :!label _label)
    (:LoopBody
      (bind _matches (CallFunction|CheckRecipeMatch Ingredients _array_element))
      (if _matches
        (Development|PrintString "GIIIIMMEEEE DIIIISHHHH")
        (return (.ResultingDish (Utilities|Struct|BreakRecipe _array_element)))
        (else
          (goto _label Break))))
    (:Completed
      (Development|PrintString "Nothing Matches")
      (return "/Game/Dish/BP_Dish.BP_Dish_C"))))

(fn CountIngredients
  (params (Array :type Array%20of%20E_IngredientType%20Enums :default "NewEnumerator0") (IngredientToCount :type E_IngredientType%20Enum :default "NewEnumerator0"))
  (for _array_element Array
    (if (Utilities|Enum|Equal(Enum) IngredientToCount _array_element)
      (Math|Integer|IncrementInt (LocalVariables|GetIngredientCount))))
  (return (LocalVariables|GetIngredientCount)))

(fn CheckRecipeMatch
  (params (Array :type Array%20of%20E_IngredientType%20Enums :default "NewEnumerator0") (Recipe :type Recipe%20Structure%20%28by%20ref%29))
  (bind _enumvalue (|ForEachE_IngredientType)
    (:LoopBody
      (bind _ingredientamount (CallFunction|CountIngredients Array _enumvalue))
      (bind _ingredientamount_2 (CallFunction|CountIngredients (.IngredientArray (Utilities|Struct|BreakRecipe Recipe)) _enumvalue))
      (if (not (== _ingredientamount _ingredientamount_2))
        (return false)))
    (:then
      (return true))))