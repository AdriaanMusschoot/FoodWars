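; BP_IngredientsDelivery is a timed spawner that periodically delivers ingredient boxes into the level.
; Tick counts DeliveryTimeLeft down and, when it drops below zero, calls SpawnAllBoxes and resets it to DeliveryTime.
; SpawnAllBoxes spawns one actor per ClassesToSpawn entry, lining them up from SpawnPoint by index times Offset.
; SpawnBox's condition is hard-wired true, so its "Not enough boxes" message never prints.
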(event EventBeginPlay
  (Variables|Default|SetDeliveryTimeLeft (Variables|Default|GetDeliveryTime)))

(event Collision|EventActorBeginOverlap
  (params (OtherActor :type Actor%20Object%20Reference)))

(event EventTick
  (params (DeltaSeconds :type Float%20%28single-precision%29))
  (bind _output_get (Variables|Default|SetDeliveryTimeLeft (- (Variables|Default|GetDeliveryTimeLeft) DeltaSeconds)))
  (if (< _output_get 0.0)
    (CallFunction|SpawnAllBoxes)
    (Variables|Default|SetDeliveryTimeLeft (Variables|Default|GetDeliveryTime))))

(fn ConstructionScript)

(fn SpawnBox
  (params (Location :type Vector) (NewParam :type BP%20Ingredient%20Box%20Class%20Reference))
  (if true
    (Game|SpawnActorfromClass NewParam (Math|Transform|MakeTransform Location) "Undefined" "MultiplyWithRoot" 0 0)
    (else
      (Development|PrintText (Utilities|Text|ToText(String) (Utilities|String|Append "Not enough boxes to spawn!" (Utilities|GetObjectName self)))))))

(fn SpawnAllBoxes
  (for (_array_element _array_index) (Variables|Default|GetClassesToSpawn)
    (CallFunction|SpawnBox (+ (* _array_index (Variables|Default|GetOffset)) (Variables|Default|GetSpawnPoint)) _array_element)))