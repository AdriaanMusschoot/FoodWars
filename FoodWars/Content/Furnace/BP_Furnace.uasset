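; BP_Furnace is an interactable cooking station that takes dropped-off ingredients and hands back cooked dishes.
; It runs a state machine of state objects, starting empty, which drive item handling, per-tick updates and delivery, each returning the next state to swap in.
; An interactible component routes drop-off and collection events, a widget shows a cook timer, and SpawnDish looks up the contents in a recipe book to spawn the dish.
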(event Custom|CustomEvent
  (params (HeldObject :type Actor%20Object%20Reference))
  (bind _asbp_ingredient (Utilities|Casting|CastToBP_Ingredient HeldObject))
  (bind _newstate (Default|HandleItem (Variables|Default|GetCurrentState) _asbp_ingredient self))
  (Utilities|IsValid _newstate
    (:Is%20Valid
      (Default|OnExit (Variables|Default|GetCurrentState) self)
      (bind _output_get (Variables|Default|SetCurrentState _newstate))
      (Default|OnEnter _output_get self)
      (Class|ActorSequenceComponent|PlaySequence (Variables|Default|GetActorSequence)))))

(event Custom|CustomEvent_0
  (bind (_newstate _dish) (Default|DeliverDish (Variables|Default|GetCurrentState) self))
  (Utilities|IsValid _newstate
    (:Is%20Valid
      (Default|OnExit (Variables|Default|GetCurrentState) self)
      (bind _output_get (Variables|Default|SetCurrentState _newstate))
      (Default|OnEnter _output_get self)
      (Variables|/Game/Furnace/BPC_Interactible.BPC_Interactible_C|SetItemToGive (Variables|Default|GetBPC_Interactible) _dish))))

(event EventBeginPlay
  (bind _bpc_interactible (Variables|Default|GetBPC_Interactible))
  (bind _returnvalue (Game|ConstructObjectfromClass "/Game/Furnace/S_FurnaceEmpty.S_FurnaceEmpty_C"))
  (Variables|Default|SetCurrentState _returnvalue)
  (bind _asbpw_timer (Utilities|Casting|CastToBPW_Timer (UserInterface|GetUserWidgetObject (Variables|Default|GetWCookTime))))
  (Variables|/Script/UMG.Widget|SetVisibility _asbpw_timer "Hidden")
  (Variables|/Game/Furnace/BPW_Timer.BPW_Timer_C|SetOwningFurnace _asbpw_timer self)
  (Variables|/Game/Furnace/BPC_Interactible.BPC_Interactible_C|SetMeshToSet (Variables|Default|GetBPC_Interactible) (Variables|Default|GetCube))
  (EventDispatchers|BindEventtoDropOffItem _bpc_interactible (delegate Custom|CustomEvent))
  (EventDispatchers|BindEventtoCollectItem _bpc_interactible (delegate Custom|CustomEvent_0)))

(event EventTick
  (params (DeltaSeconds :type Float%20%28single-precision%29))
  (bind _newstate (Default|Update (Variables|Default|GetCurrentState) DeltaSeconds self))
  (Utilities|IsValid _newstate
    (:Is%20Valid
      (Default|OnExit (Variables|Default|GetCurrentState) self)
      (bind _output_get (Variables|Default|SetCurrentState _newstate))
      (Default|OnEnter _output_get self))))

(fn ConstructionScript)

(fn SpawnDish
  (bind _recipebook (Variables|Default|GetRecipeBook))
  (Utilities|IsValid _recipebook
    (:Is%20Valid
      (bind _dish (Default|GetDish _recipebook (Variables|Default|GetContents)))
      (bind _returnvalue (Game|SpawnActorfromClass _dish (Math|Transform|MakeTransform "0, 0, 0" "0, 0, 0" "1.000000,1.000000,1.000000") "AlwaysSpawn" "MultiplyWithRoot" 0 0))
      (return _returnvalue))))